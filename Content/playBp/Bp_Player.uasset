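; Player character Blueprint handling third-person camera look and WASD movement.
; Each Tick, input axes rotate the spring arm, and the mesh follows its yaw.
; Movement keys set yaw offsets that are summed with camera yaw into a forward vector for AddMovementInput while Move is true.
; Any press sets Move; releasing W, A or D clears it, but releasing S only resets its offset.
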(event `self.ReceiveTick`
  (params (DeltaSeconds :type "Float (single-precision)"))
  (bind _springarm (`self.SpringArm`))
  (bind (_returnvalue_roll _returnvalue_pitch _returnvalue_yaw) (`KismetMathLibrary.BreakRotator` (`SceneComponent.K2_GetComponentRotation` (`self.SpringArm`))))
  (bind (_returnvalue_roll_2 _returnvalue_pitch_2 _returnvalue_yaw_2) (`KismetMathLibrary.BreakRotator` (`SceneComponent.K2_GetComponentRotation` _springarm)))
  (bind _returnvalue (+ _returnvalue_yaw_2 (`self.GetInputAxisKeyValue`)))
  (`SceneComponent.K2_SetWorldRotation` _springarm (`KismetMathLibrary.MakeRotator` 0.0 (+ _returnvalue_pitch_2 (`self.GetInputAxisKeyValue`)) _returnvalue) false false)
  (`SceneComponent.K2_SetWorldRotation` (`self.Mesh`) (`KismetMathLibrary.MakeRotator` 0.0 0.0 _returnvalue) false false)
  (set `self.방향` (`KismetMathLibrary.GetForwardVector` (`KismetMathLibrary.MakeRotator` 0.0 0.0 (+ _returnvalue_yaw (`self.w`) (`self.a`) (`self.s`) (`self.d`)))))
  (if (`self.move`)
    (`self.AddMovementInput` (`self.방향`) 10.0)))

(event `Key|W`
  (params (Key :type "Key Structure"))
  (:`Pressed`
    (set `self.w` 0.0)
    (set `self.move` true :!label _label))
  (:`Released`
    (set `self.w` 0.0)
    (set `self.move` false :!label _label_2)))

(event `Key|S`
  (params (Key :type "Key Structure"))
  (:`Pressed`
    (set `self.s` (+ 0.0 180.0))
    (goto _label))
  (:`Released`
    (set `self.s` 0.0)))

(event `Key|D`
  (params (Key :type "Key Structure"))
  (:`Pressed`
    (set `self.d` (+ 0.0 90.0))
    (goto _label))
  (:`Released`
    (set `self.d` 0.0)
    (goto _label_2)))

(event `Key|A`
  (params (Key :type "Key Structure"))
  (:`Pressed`
    (set `self.a` (+ 0.0 270.0))
    (goto _label))
  (:`Released`
    (set `self.a` 0.0)
    (goto _label_2)))

(fn `UserConstructionScript`)